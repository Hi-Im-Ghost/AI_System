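; NPC character driven by four needs (Energy, Food, Happy, Cash), with a melee punch against the third-person character.
; A random trait or random defaults set need weights at spawn, alongside random tints.
; Needs decay on Tick, and a looping timer ranks them lowest-first into Blackboard queue keys.
; Overlapping the current point refills its need on a timer and pauses that decay, while punches sphere-trace on a montage notify.
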(event OnComponentBeginOverlap(CapsuleComponent)
  (params (OverlappedComponent :type Primitive%20Component%20Object%20Reference) (OtherActor :type Actor%20Object%20Reference) (OtherComp :type Primitive%20Component%20Object%20Reference) (OtherBodyIndex :type Integer) (bFromSweep :type Boolean) (SweepResult :type Hit%20Result%20Structure%20%28by%20ref%29))
  ;[0 1 0.223] Zwiekszanie wartosci zmiennych potrzeb
  (bind _output_get (Variables|Default|SetOverlapActor OtherActor))
  (if (== _output_get (Variables|Default|GetCurrentPoint))
    (bind _returnvalue (Utilities|Time|SetTimerbyEvent (delegate Custom|IncreaseNeedsValue) 1.0 true))
    (Variables|Default|SetTimer _returnvalue)))

(event OnComponentEndOverlap(CapsuleComponent)
  (params (OverlappedComponent :type Primitive%20Component%20Object%20Reference) (OtherActor :type Actor%20Object%20Reference) (OtherComp :type Primitive%20Component%20Object%20Reference) (OtherBodyIndex :type Integer))
  ;[0 1 0.223] Zwiekszanie wartosci zmiennych potrzeb
  (Utilities|Time|ClearandInvalidateTimerbyHandle (Variables|Default|GetTimer))
  (Variables|Default|SetOverlapActor 0)
  (Variables|Default|SetStopSubstract false))

(event Custom|IncreaseNeedsValue
  (bind _currentpoint (Variables|Default|GetCurrentPoint))
  (bind _npc_needs (Variables|Default|GetNPC%20Needs))
  (bind _npc_needs_2 (Variables|Default|GetNPC%20Needs))
  (bind _textrender (Variables|Default|GetTextRender))
  (bind _value (Utilities|Map|Find (.needs _npc_needs_2) "Energy"))
  (bind _value_2 (Utilities|Map|Find (.needs _npc_needs_2) "Food"))
  (bind _value_3 (Utilities|Map|Find (.needs _npc_needs_2) "Happy"))
  (bind _value_4 (Utilities|Map|Find (.needs _npc_needs_2) "Cash"))
  ;[0 1 0.223] Zwiekszanie wartosci zmiennych potrzeb
  (if (== (Variables|Default|GetOverlapActor) _currentpoint)
    (switch Utilities|FlowControl|Switch|SwitchonObjectTypeList (Variables|/Game/Points/PointPath.PointPath_C|GetObjectType _currentpoint)
      (:NewEnumerator0
        (if (< _value 1e+02)
          (Variables|Default|SetStopSubstract true)
          (Utilities|Map|Add (.needs _npc_needs) "Energy" (Math|Float|Clamp(Float) (+ _value (.Value (Utilities|Map|Find (.weightincreasing (.detail _npc_needs_2)) "Energy"))) 0.0 1e+02))
          (Rendering|Components|TextRender|SetText _textrender (Utilities|Text|MakeLiteralText "Odnawia energie"))))
      (:NewEnumerator1
        (if (< _value_2 1e+02)
          (Variables|Default|SetStopSubstract true)
          (Utilities|Map|Add (.needs _npc_needs) "Food" (Math|Float|Clamp(Float) (+ _value_2 (.Value (Utilities|Map|Find (.weightincreasing (.detail _npc_needs_2)) "Food"))) 0.0 1e+02))
          (Rendering|Components|TextRender|SetText _textrender (Utilities|Text|MakeLiteralText "Odnawia jedzenie"))))
      (:NewEnumerator2
        (if (< _value_3 1e+02)
          (Variables|Default|SetStopSubstract true)
          (Utilities|Map|Add (.needs _npc_needs) "Happy" (Math|Float|Clamp(Float) (+ _value_3 (.Value (Utilities|Map|Find (.weightincreasing (.detail _npc_needs_2)) "Happy"))) 0.0 1e+02))
          (Rendering|Components|TextRender|SetText _textrender (Utilities|Text|MakeLiteralText "Odnawia zadowolenie"))))
      (:NewEnumerator3
        (if (< _value_4 1e+02)
          (Variables|Default|SetStopSubstract true)
          (Utilities|Map|Add (.needs _npc_needs) "Cash" (Math|Float|Clamp(Float) (+ _value_4 (.Value (Utilities|Map|Find (.weightincreasing (.detail _npc_needs_2)) "Cash"))) 0.0 1e+02))
          (Rendering|Components|TextRender|SetText _textrender (Utilities|Text|MakeLiteralText "Odnawia pieniadze")))))))

(event Custom|SetQueueNeeds
  (bind _returnvalue (AI|GetBlackboard 0))
  (bind _npc_needs (Variables|Default|GetNPC%20Needs))
  (bind _queueneeds (Variables|Default|GetQueueNeeds))
  ;[1 0.7303 0.492] Tworzenie i aktualizacja kolejki potrzeb
  (bind _keys (Utilities|Map|Keys (.needs _npc_needs)))
  (Variables|Default|SetNeedsKeys _keys)
  (bind _values (Utilities|Map|Values (.needs _npc_needs)))
  (bind _output_get (Variables|Default|SetNeedsValues _values))
  (Variables|Default|SetIndex 0)
  (while (> (Utilities|Array|Length _output_get) 0)
    (bind _result (Math|Integer|IncrementInt (Variables|Default|GetIndex))
      (:%20%20
        (Utilities|Map|Add (Variables|Default|GetQueueNeeds) (Utilities|Array|Get(acopy) (Variables|Default|GetNeedsKeys) (.IndexOfMinValue (Math|Float|MinOfFloatArray (Variables|Default|GetNeedsValues)))) _result)
        (Utilities|Array|RemoveIndex (Variables|Default|GetNeedsKeys) (.IndexOfMinValue (Math|Float|MinOfFloatArray (Variables|Default|GetNeedsValues))))
        (Utilities|Array|RemoveIndex (Variables|Default|GetNeedsValues) (.IndexOfMinValue (Math|Float|MinOfFloatArray (Variables|Default|GetNeedsValues)))))))
  (bind _keys_2 (Utilities|Map|Keys _queueneeds))
  (bind _values_2 (Utilities|Map|Values _queueneeds))
  (for (_array_element _array_index) _values_2
    (switch int _array_element
      (:1
        (Class|BlackboardComponent|SetValueasName _returnvalue (Utilities|Name|MakeLiteralName "Q1Need") (Utilities|Array|Get(acopy) _keys_2 _array_index)))
      (:2
        (Class|BlackboardComponent|SetValueasName _returnvalue (Utilities|Name|MakeLiteralName "Q2Need") (Utilities|Array|Get(acopy) _keys_2 _array_index)))
      (:3
        (Class|BlackboardComponent|SetValueasName _returnvalue (Utilities|Name|MakeLiteralName "Q3Need") (Utilities|Array|Get(acopy) _keys_2 _array_index)))
      (:4
        (Class|BlackboardComponent|SetValueasName _returnvalue (Utilities|Name|MakeLiteralName "Q4Need") (Utilities|Array|Get(acopy) _keys_2 _array_index))))))

(event EventBeginPlay
  (bind _returnvalue (Math|Random|RandomFloat))
  (bind _returnvalue_2 (Math|Random|RandomFloat))
  (bind _returnvalue_3 (Math|Random|RandomFloat))
  (bind _traitscomponent (Variables|Default|GetTraitsComponent))
  (bind _returnvalue_4 (Math|Color|MakeColor _returnvalue _returnvalue_2 _returnvalue_3))
  (bind _traits (Variables|/Game/Traits/TraitsComponent.TraitsComponent_C|GetTraits _traitscomponent))
  (bind _returnvalue_5 (Utilities|Map|Length _traits))
  (bind _returnvalue_6 (Math|Random|RandomInteger _returnvalue_5))
  (bind (_value _returnvalue_7) (Utilities|Map|Find _traits _returnvalue_6))
  ;[1 0.9452 0] Ustawienie poczatkowe wartosci potrzeb, losowanie cech, losowanie i przypisanie koloru cialu postaci
  (bind _returnvalue_8 (Utilities|Time|SetTimerbyEvent (delegate Custom|SetQueueNeeds) 5.0 true))
  (Variables|Default|SetTimerForQueueNeeds _returnvalue_8)
  (Default|SetHealth (Variables|Default|GetHealthComponent) 1e+02)
  (CallFunction|SetNeedsPoints)
  (if _returnvalue_7
    (Default|SetActivTrait _traitscomponent _value)
    (bind _trait (Default|GetActivTrait (Variables|Default|GetTraitsComponent)))
    (CallFunction|SetNeedsValuewithTrait _trait)
    (else
      (CallFunction|SetDefaultNeedsValue)))
  (bind _returnvalue_9 (Rendering|Material|CreateDynamicMaterialInstance (Variables|Character|GetMesh) 0 0 "None" :!class /Script/Engine.PrimitiveComponent))
  (Rendering|Material|SetVectorParameterValue _returnvalue_9 "Tint" _returnvalue_4 :!class /Script/Engine.MaterialInstanceDynamic)
  (Rendering|Components|TextRender|SetTextRenderColor (Variables|Default|GetTextRender) (Math|Conversions|ToColor(LinearColor) _returnvalue_4)))

(event EventMeleeAttack
  (bind _self self)
  (bind _mesh (Variables|Character|GetMesh))
  (bind _returnvalue (Transformation|GetSocketLocation _mesh "R_Punch"))
  (bind _charactermovement (Variables|Character|GetCharacterMovement _self))
  ;[1 0 0.1167 1 20] System walki
  (Utilities|IsValid _charactermovement
    (:Is%20Valid
      (Pawn|Components|CharacterMovement|DisableMovement _charactermovement)
      (Animation|Montage|PlayMontage _mesh "/Game/Anim/HookPunch_UE_Montage.HookPunch_UE_Montage"
        (:OnCompleted
          (Utilities|IsValid _charactermovement :!label _label
            (:Is%20Valid
              (Pawn|Components|CharacterMovement|SetMovementMode _charactermovement "MOVE_Walking" 0))))
        (:OnInterrupted
          (goto _label))
        (:OnNotifyBegin
          (bind _outhit (Collision|SphereTraceByChannel _returnvalue (+ _returnvalue (* (Math|Vector|GetForwardVector (Transformation|GetActorRotation)) 7.0)) 1e+01 "TraceTypeQuery2" false 0 "ForDuration"))
          (bind _asbp_third_person_character (Utilities|Casting|CastToBP_ThirdPersonCharacter (.hitactor _outhit)))
          (if (Variables|/Script/Engine.Actor|GetbCanBeDamaged _asbp_third_person_character)
            (Class|AISenseDamage|ReportDamageEvent (.hitactor _outhit) self 2e+01 (.tracestart _outhit) (.location _outhit) "None")
            (Game|Damage|ApplyDamage (.hitactor _outhit) 2e+01 0 0)))))))

(event EventTick
  (params (DeltaSeconds :type Float%20%28single-precision%29))
  ;[0.02628 0.4395 1] Zmniejszanie wartosci zmiennych potrzeb w czasie delta
  (CallFunction|SubstractValueNeeds DeltaSeconds))

(fn ConstructionScript
  (|CallParentFunction))

(fn SubstractValueNeeds
  (params (Delta%20Seconds :type Float%20%28double-precision%29))
  (if (Variables|Default|GetStopSubstract)
    (switch Utilities|FlowControl|Switch|SwitchonObjectTypeList (Variables|/Game/Points/PointPath.PointPath_C|GetObjectType (Variables|Default|GetCurrentPoint))
      (:NewEnumerator0
        (Variables|Default|SetNPC%20Needs (Utilities|Struct|MakeNPC_Needs (Utilities|Map|MakeMap "Energy" (.Value (Utilities|Map|Find (.needs (Variables|Default|GetNPC%20Needs)) "Energy")) "Food" (Math|Float|Clamp(Float) (- (.Value (Utilities|Map|Find (.needs (Variables|Default|GetNPC%20Needs)) "Food")) (* Delta%20Seconds (.Value (Utilities|Map|Find (.weightsubtraction (.detail (Variables|Default|GetNPC%20Needs))) "Food")))) 0.0 1e+02) "Happy" (Math|Float|Clamp(Float) (- (.Value (Utilities|Map|Find (.needs (Variables|Default|GetNPC%20Needs)) "Happy")) (* Delta%20Seconds (.Value (Utilities|Map|Find (.weightsubtraction (.detail (Variables|Default|GetNPC%20Needs))) "Happy")))) 0.0 1e+02) "Cash" (Math|Float|Clamp(Float) (- (.Value (Utilities|Map|Find (.needs (Variables|Default|GetNPC%20Needs)) "Cash")) (* Delta%20Seconds (.Value (Utilities|Map|Find (.weightsubtraction (.detail (Variables|Default|GetNPC%20Needs))) "Cash")))) 0.0 1e+02)) (.detail (Variables|Default|GetNPC%20Needs)))))
      (:NewEnumerator1
        (Variables|Default|SetNPC%20Needs (Utilities|Struct|MakeNPC_Needs (Utilities|Map|MakeMap "Energy" (Math|Float|Clamp(Float) (- (.Value (Utilities|Map|Find (.needs (Variables|Default|GetNPC%20Needs)) "Energy")) (* Delta%20Seconds (.Value (Utilities|Map|Find (.weightsubtraction (.detail (Variables|Default|GetNPC%20Needs))) "Energy")))) 0.0 1e+02) "Food" (.Value (Utilities|Map|Find (.needs (Variables|Default|GetNPC%20Needs)) "Food")) "Happy" (Math|Float|Clamp(Float) (- (.Value (Utilities|Map|Find (.needs (Variables|Default|GetNPC%20Needs)) "Happy")) (* Delta%20Seconds (.Value (Utilities|Map|Find (.weightsubtraction (.detail (Variables|Default|GetNPC%20Needs))) "Happy")))) 0.0 1e+02) "Cash" (Math|Float|Clamp(Float) (- (.Value (Utilities|Map|Find (.needs (Variables|Default|GetNPC%20Needs)) "Cash")) (* Delta%20Seconds (.Value (Utilities|Map|Find (.weightsubtraction (.detail (Variables|Default|GetNPC%20Needs))) "Cash")))) 0.0 1e+02)) (.detail (Variables|Default|GetNPC%20Needs)))))
      (:NewEnumerator2
        (Variables|Default|SetNPC%20Needs (Utilities|Struct|MakeNPC_Needs (Utilities|Map|MakeMap "Energy" (Math|Float|Clamp(Float) (- (.Value (Utilities|Map|Find (.needs (Variables|Default|GetNPC%20Needs)) "Energy")) (* Delta%20Seconds (.Value (Utilities|Map|Find (.weightsubtraction (.detail (Variables|Default|GetNPC%20Needs))) "Energy")))) 0.0 1e+02) "Food" (Math|Float|Clamp(Float) (- (.Value (Utilities|Map|Find (.needs (Variables|Default|GetNPC%20Needs)) "Food")) (* Delta%20Seconds (.Value (Utilities|Map|Find (.weightsubtraction (.detail (Variables|Default|GetNPC%20Needs))) "Food")))) 0.0 1e+02) "Happy" (.Value (Utilities|Map|Find (.needs (Variables|Default|GetNPC%20Needs)) "Happy")) "Cash" (Math|Float|Clamp(Float) (- (.Value (Utilities|Map|Find (.needs (Variables|Default|GetNPC%20Needs)) "Cash")) (* Delta%20Seconds (.Value (Utilities|Map|Find (.weightsubtraction (.detail (Variables|Default|GetNPC%20Needs))) "Cash")))) 0.0 1e+02)) (.detail (Variables|Default|GetNPC%20Needs)))))
      (:NewEnumerator3
        (Variables|Default|SetNPC%20Needs (Utilities|Struct|MakeNPC_Needs (Utilities|Map|MakeMap "Energy" (Math|Float|Clamp(Float) (- (.Value (Utilities|Map|Find (.needs (Variables|Default|GetNPC%20Needs)) "Energy")) (* Delta%20Seconds (.Value (Utilities|Map|Find (.weightsubtraction (.detail (Variables|Default|GetNPC%20Needs))) "Energy")))) 0.0 1e+02) "Food" (Math|Float|Clamp(Float) (- (.Value (Utilities|Map|Find (.needs (Variables|Default|GetNPC%20Needs)) "Food")) (* Delta%20Seconds (.Value (Utilities|Map|Find (.weightsubtraction (.detail (Variables|Default|GetNPC%20Needs))) "Food")))) 0.0 1e+02) "Happy" (Math|Float|Clamp(Float) (- (.Value (Utilities|Map|Find (.needs (Variables|Default|GetNPC%20Needs)) "Happy")) (* Delta%20Seconds (.Value (Utilities|Map|Find (.weightsubtraction (.detail (Variables|Default|GetNPC%20Needs))) "Happy")))) 0.0 1e+02) "Cash" (.Value (Utilities|Map|Find (.needs (Variables|Default|GetNPC%20Needs)) "Cash"))) (.detail (Variables|Default|GetNPC%20Needs))))))
    (else
      (Variables|Default|SetNPC%20Needs (Utilities|Struct|MakeNPC_Needs (Utilities|Map|MakeMap "Energy" (Math|Float|Clamp(Float) (- (.Value (Utilities|Map|Find (.needs (Variables|Default|GetNPC%20Needs)) "Energy")) (* Delta%20Seconds (.Value (Utilities|Map|Find (.weightsubtraction (.detail (Variables|Default|GetNPC%20Needs))) "Energy")))) 0.0 1e+02) "Food" (Math|Float|Clamp(Float) (- (.Value (Utilities|Map|Find (.needs (Variables|Default|GetNPC%20Needs)) "Food")) (* Delta%20Seconds (.Value (Utilities|Map|Find (.weightsubtraction (.detail (Variables|Default|GetNPC%20Needs))) "Food")))) 0.0 1e+02) "Happy" (Math|Float|Clamp(Float) (- (.Value (Utilities|Map|Find (.needs (Variables|Default|GetNPC%20Needs)) "Happy")) (* Delta%20Seconds (.Value (Utilities|Map|Find (.weightsubtraction (.detail (Variables|Default|GetNPC%20Needs))) "Happy")))) 0.0 1e+02) "Cash" (Math|Float|Clamp(Float) (- (.Value (Utilities|Map|Find (.needs (Variables|Default|GetNPC%20Needs)) "Cash")) (* Delta%20Seconds (.Value (Utilities|Map|Find (.weightsubtraction (.detail (Variables|Default|GetNPC%20Needs))) "Cash")))) 0.0 1e+02)) (.detail (Variables|Default|GetNPC%20Needs)))))))

(fn SetNeedsPoints
  (bind _outactors (Actor|GetAllActorsOfClass "/Game/Points/PointEnergy.PointEnergy_C"))
  (bind _outactors_2 (Actor|GetAllActorsOfClass "/Game/Points/PointFood.PointFood_C"))
  (bind _outactors_3 (Actor|GetAllActorsOfClass "/Game/Points/PointHappy.PointHappy_C"))
  (bind _outactors_4 (Actor|GetAllActorsOfClass "/Game/Points/PointWork.PointWork_C"))
  (Variables|Default|SetPathPoint (Utilities|Struct|MakePointType _outactors _outactors_2 _outactors_3 _outactors_4)))

(fn SetDefaultNeedsValue
  (bind _returnvalue (Math|Random|RandomFloatinRange 4.0 1e+01))
  (bind _returnvalue_2 (Math|Random|RandomFloatinRange 5.0 3e+01))
  (bind _returnvalue_3 (Math|Random|RandomFloatinRange 0.1 1.0))
  (Variables|Default|SetNPC%20Needs (Utilities|Struct|MakeNPC_Needs (Utilities|Map|MakeMap "Energy" (Math|Random|RandomFloatinRange 8e+01 1e+02) "Food" (Math|Random|RandomFloatinRange 5e+01 1e+02) "Happy" (Math|Random|RandomFloatinRange 4e+01 1e+02) "Cash" (Math|Random|RandomFloatinRange 2e+01 1e+02)) (Utilities|Struct|MakeNeedDetailStructure (Utilities|Map|MakeMap 1 "Energy" 2 "Food" 3 "Happy" 4 "Cash") (Utilities|Map|MakeMap "Energy" _returnvalue_2 "Food" _returnvalue_2 "Happy" _returnvalue_2 "Cash" _returnvalue_2) (Utilities|Map|MakeMap "Energy" _returnvalue_3 "Food" _returnvalue_3 "Happy" _returnvalue_3 "Cash" _returnvalue_3) (Utilities|Map|MakeMap "Energy" _returnvalue "Food" _returnvalue "Happy" _returnvalue "Cash" _returnvalue)))))

(fn SetNeedsValuewithTrait
  (params (Trait :type Name))
  (bind _returnvalue (Utilities|GetDataTableRow "/Game/Traits/TraitsDataTable.TraitsDataTable" Trait)
    (:then
      (Variables|Default|SetNPC%20Needs (Utilities|Struct|MakeNPC_Needs (Utilities|Map|MakeMap "Energy" (Math|Random|RandomFloatinRange 8e+01 1e+02) "Food" (Math|Random|RandomFloatinRange 5e+01 1e+02) "Happy" (Math|Random|RandomFloatinRange 4e+01 1e+02) "Cash" (Math|Random|RandomFloatinRange 2e+01 1e+02)) (.detail _returnvalue))))))