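; BP_BaseAI is a base AI character Blueprint that handles damage and death.
; AnyDamage passes damage through HealthComponent and, once dead, ragdolls the mesh, stops the AI controller's behavior logic, disables capsule collision and destroys the actor after a delay.
; A StopMontage event halts the currently playing montage immediately via both the AnimInstance and the character.
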(event Custom|StopMontage
  (bind _returnvalue (Animation|GetCurrentMontage :!class /Script/Engine.Character))
  ;[1 0.1931 0.8758] Wydarzenie zatrzymujace aktualnie odtwarzana animacje
  (Animation|Montage|MontageStop (Components|SkeletalMesh|GetAnimInstance (Variables|Character|GetMesh self)) 0.0 _returnvalue)
  (Animation|StopAnimMontage self _returnvalue))

(event Game|Damage|EventAnyDamage
  (params (Damage :type Float%20%28single-precision%29) (DamageType :type Damage%20Type%20Object%20Reference) (InstigatedBy :type Controller%20Object%20Reference) (DamageCauser :type Actor%20Object%20Reference))
  (bind _healthcomponent (Variables|Default|GetHealthComponent))
  ;[1 0.1096 0.1993] Obsluga otrzymania obrazen
  (bind _health (Default|TakeDamage _healthcomponent Damage))
  (Default|SetHealth _healthcomponent _health)
  (if (Variables|/Game/Components/HealthComponent.HealthComponent_C|GetisDead _healthcomponent)
    (Physics|SetSimulatePhysics (Variables|Character|GetMesh) true)
    (AI|Logic|StopLogic (Variables|/Script/AIModule.AIController|GetBrainComponent (AI|GetAIController self)) "Dead")
    (Collision|SetCollisionEnabled (Variables|Collision|GetCapsuleComponent) "NoCollision")
    (Utilities|FlowControl|Delay 1e+01)
    (Actor|DestroyActor)))

(fn ConstructionScript)